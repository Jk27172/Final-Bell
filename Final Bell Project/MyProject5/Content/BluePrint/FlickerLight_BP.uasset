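; A spotlight actor that randomly flickers with a buzzing sound, like a faulty light.
; A looping timer started on BeginPlay either rolls a chance to begin a flicker or, during one, sets intensity to a random fraction range of the base value.
; Each flicker plays the buzz at a random pitch, then a one-shot timer stops the sound and restores base intensity.
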(event Custom|UpdateFlicker
  (if (Variables|Default|GetbIsFlickering)
    (Rendering|Components|Light|SetIntensity (Variables|Default|GetSpotLight) (* (Math|Random|RandomFloatinRange (Variables|Default|GetMinFlicker) (Variables|Default|GetMaxFlicker)) (Variables|Default|GetBaseIntensity)))
    (elif (< (Math|Random|RandomFloatinRange 0.0 1.0) (Variables|Default|GetFlickerChance))
      (Variables|Default|SetbIsFlickering true)
      (Audio|Components|Audio|SetPitchMultiplier (Variables|Default|GetBuzzingSound) (Math|Random|RandomFloatinRange 0.9 1.1))
      (Audio|Components|Audio|Play (Variables|Default|GetBuzzingSound) 0.0)
      (Utilities|Time|SetTimerbyEvent (delegate Custom|StopFlicker) (Variables|Default|GetFlickerDuration)))))

(event Custom|StopFlicker
  (Variables|Default|SetbIsFlickering false)
  (Audio|Components|Audio|Stop (Variables|Default|GetBuzzingSound))
  (Rendering|Components|Light|SetIntensity (Variables|Default|GetSpotLight) (Variables|Default|GetBaseIntensity)))

(event EventBeginPlay
  (Utilities|Time|SetTimerbyEvent (delegate Custom|UpdateFlicker) 0.1 true))

(event Collision|EventActorBeginOverlap
  (params (OtherActor :type Actor%20Object%20Reference)))

(event EventTick
  (params (DeltaSeconds :type Float%20%28single-precision%29)))

(fn ConstructionScript)