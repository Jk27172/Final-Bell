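; BP_ZombieSpawner spawns a set number of BP_Zombie actors at random spawn points in the level.
; SpawnZombies gathers all BP_ZombieSpawnPoint actors, shuffles them and takes one point per zombie up to ZombiesToSpawn, without checking the point count.
; Each zombie spawns slightly above its point with random yaw, adjusting for collision but always spawning.
; BeginPlay is empty, and nothing in this Blueprint calls SpawnZombies.
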(event Custom|SpawnZombies
  ;[0.15 0.15 0.15 0.5] // Spawn Zombies
  (bind _outactors (Actor|GetAllActorsOfClass "/Game/BluePrint/BP_ZombieSpawnPoint.BP_ZombieSpawnPoint_C"))
  (Utilities|Array|Shuffle _outactors)
  (for _index (range 0 (- (Variables|Default|GetZombiesToSpawn) 1))
    (Game|SpawnActorfromClass "/Game/BluePrint/BP_Zombie.BP_Zombie_C" (Math|Transform|MakeTransform (+ (Transformation|GetActorLocation (Utilities|Array|Get(acopy) _outactors _index)) (Math|Vector|MakeVector 0.0 0.0 1e+02)) (Math|Rotator|MakeRotator 0.0 0.0 (Math|Random|RandomFloatinRange 0.0 3.6e+02))) "AdjustIfPossibleButAlwaysSpawn" "MultiplyWithRoot" 0 0)))

(event EventBeginPlay)

(fn ConstructionScript)