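; BP_Zombie is a melee enemy character that attacks the player, takes damage and dies.
; StartAttack freezes movement for a timed montage, while DealDamageToPlayer checks range and line trace before applying damage.
; AnyDamage lowers health, triggers hit reactions and briefly shows a camera-facing health bar.
; Die disables collision, stops the AI controller's chase and sets a lifespan, though its montage and cleanup, like hit reactions, require valid attack audio.
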(event Custom|StartAttack
  ;[0.15 0.15 0.15 0.5] // Start & Reset Attack
  (Variables|Default|SetDidHitThisAttack false)
  (if (Math|Boolean|ANDBoolean (not (Variables|Default|GetIsDead)) (not (Variables|Default|GetIsAttacking)) (not (Variables|Default|GetIsHitReacting)))
    (Variables|Default|SetIsAttacking true)
    (Variables|Default|SetDidHitThisAttack false)
    (Pawn|Components|CharacterMovement|DisableMovement (Variables|Character|GetCharacterMovement))
    (bind _returnvalue (Animation|PlayAnimMontage "/Game/ZombieCharacter/ZombieAnimation/Scary_Zombie_Pack/AM_ZombieAttack.AM_ZombieAttack" 1.0 "None"))
    (Utilities|Time|SetTimerbyEvent (EventDispatchers|CreateEvent :!event Custom|ResetAttack) (+ _returnvalue 0.2))))

(event Custom|ResetAttack
  ;[0.15 0.15 0.15 0.5] // Start & Reset Attack
  (Components|Movement|StopMovementImmediately (Variables|Character|GetCharacterMovement))
  (Pawn|Components|CharacterMovement|SetMovementMode (Variables|Character|GetCharacterMovement) "MOVE_Walking" 0)
  (Variables|Default|SetIsAttacking false)
  (Variables|Default|SetDidHitThisAttack false))

(event Custom|DealDamageToPlayer
  (bind _returnvalue (Game|GetPlayerCharacter 0))
  (bind _returnvalue_2 (Transformation|GetActorLocation))
  (bind _returnvalue_3 (Transformation|GetActorLocation _returnvalue))
  ;[0.15 0.15 0.15 0.5] // Damage To Player Event
  (if (not (Variables|Default|GetIsDead))
    (if (<= (Math|Vector|Distance(Vector) _returnvalue_2 _returnvalue_3) (Variables|Default|GetAttackRange))
      (bind _outhit (Collision|LineTraceByChannel _returnvalue_2 _returnvalue_3 "TraceTypeQuery3" false 0 "None"))
      (if (== (.HitActor (Collision|BreakHitResult _outhit)) _returnvalue)
        (bind _asbp_third_person_character (Utilities|Casting|CastToBP_ThirdPersonCharacter _returnvalue))
        (if (not (Variables|/Game/ThirdPerson/Blueprints/BP_ThirdPersonCharacter.BP_ThirdPersonCharacter_C|GetisDead _asbp_third_person_character))
          (Game|Damage|ApplyDamage _returnvalue (Variables|Default|GetAttackDamage) (Pawn|GetController) self))))))

(event Custom|Die
  (bind _capsulecomponent (Variables|Collision|GetCapsuleComponent))
  (bind _mesh (Variables|Character|GetMesh))
  (bind _attackaudiocomponent (Variables|Default|GetAttackAudioComponent))
  ;[0.15 0.15 0.15 0.5] // Die Event
  (if (not (Variables|Default|GetIsDead))
    (Variables|Default|SetIsDead true)
    (Collision|SetCollisionEnabled _capsulecomponent "NoCollision")
    (Variables|/Script/Engine.PrimitiveComponent|SetbGenerateOverlapEvents _capsulecomponent false)
    (Collision|SetCollisionEnabled _mesh "NoCollision")
    (Physics|SetSimulatePhysics _mesh false)
    (Utilities|IsValid _attackaudiocomponent
      (:Is%20Valid
        (Audio|Components|Audio|Stop _attackaudiocomponent)
        (bind _asbp_zombie_aicontroller (Utilities|Casting|CastToBP_ZombieAIController (Pawn|GetController)))
        (Utilities|Time|ClearandInvalidateTimerbyHandle (Variables|/Game/BluePrint/BP_ZombieAIController.BP_ZombieAIController_C|GetChaseTimerHandle _asbp_zombie_aicontroller))
        (AI|Navigation|StopMovement _asbp_zombie_aicontroller)
        (Pawn|Components|CharacterMovement|DisableMovement (Variables|Character|GetCharacterMovement))
        (Components|Movement|StopMovementImmediately (Variables|Character|GetCharacterMovement))
        (Animation|PlayAnimMontage "/Game/ZombieCharacter/ZombieAnimation/Scary_Zombie_Pack/AM_ZombieDie.AM_ZombieDie" 1.0 "None")
        (Utilities|FlowControl|Delay 1.2)
        (Actor|SetLifeSpan 4.0)
        (Rendering|SetVisibility (Variables|Default|GetHealthWidget) false false)))))

(event Custom|PlayAttackSound
  ;[0.15 0.15 0.15 0.5] // Attack Sound
  (bind _returnvalue (Audio|SpawnSoundAttached "/Game/Import/Sound/freesound_community-zombie-attack-6419.freesound_community-zombie-attack-6419" (Variables|Character|GetMesh) "None" "0, 0, 0" "0, 0, 0" "KeepRelativeOffset" false 1.0 (Math|Random|RandomFloatinRange 0.9 1.05) 0.0 0 0 false))
  (Variables|Default|SetAttackAudioComponent _returnvalue))

(event Custom|HideHealthBar
  ;[0.15 0.15 0.15 0.5] // Health Bar Visibility
  (Rendering|SetVisibility (Variables|Default|GetHealthWidget) false false))

(event Custom|HitReact
  (bind _attackaudiocomponent (Variables|Default|GetAttackAudioComponent))
  ;[0.15 0.15 0.15 0.5] // Hit React Event
  (if (not (Variables|Default|GetIsDead))
    (if (and (not (Variables|Default|GetIsDead)) (not (Variables|Default|GetIsHitReacting)))
      (Utilities|IsValid _attackaudiocomponent
        (:Is%20Valid
          (Audio|Components|Audio|Stop _attackaudiocomponent)
          (Variables|Default|SetIsHitReacting true)
          (Variables|Default|SetIsAttacking false)
          (Components|Movement|StopMovementImmediately (Variables|Character|GetCharacterMovement))
          (Animation|PlayAnimMontage "/Game/ZombieCharacter/ZombieAnimation/Scary_Zombie_Pack/AM_ZombieHit.AM_ZombieHit" 1.0 "None")
          (Audio|PlaySoundatLocation (Variables|Default|GetHitReactSound) (Transformation|GetActorLocation) "0, 0, 0" 1.0 1.0 0.0 0 0 0 0)
          (Utilities|Time|SetTimerbyEvent (EventDispatchers|CreateEvent :!event Custom|EndHitReact) (Variables|Default|GetHitReactDuration)))))))

(event Custom|EndHitReact
  ;[0.15 0.15 0.15 0.5] // Hit React Event
  (Variables|Default|SetIsHitReacting false))

(event Game|Damage|EventAnyDamage
  (params (Damage :type Float%20%28single-precision%29) (DamageType :type Damage%20Type%20Object%20Reference) (InstigatedBy :type Controller%20Object%20Reference) (DamageCauser :type Actor%20Object%20Reference))
  ;[0.15 0.15 0.15 0.5] // Health Bar Visibility
  (if (not (Variables|Default|GetIsDead))
    (CallFunction|ApplyHealthDamage (* Damage -1.0))
    (CallFunction|HitReact)
    (Rendering|SetVisibility (Variables|Default|GetHealthWidget) true true)
    (Utilities|Time|ClearandInvalidateTimerbyHandle (Variables|Default|GetHideHealthBarTimer))
    (bind _returnvalue (Utilities|Time|SetTimerbyEvent (EventDispatchers|CreateEvent :!event Custom|HideHealthBar) (Variables|Default|GetHealthBarVisibleTime)))
    (Variables|Default|SetHideHealthBarTimer _returnvalue)))

(event EventBeginPlay
  ;[0.15 0.15 0.15 0.5] // Event Begin Play
  (Utilities|FlowControl|Sequence
    (:then_0
      (bind _aswbp_zombie_health (Utilities|Casting|CastToWBP_ZombieHealth (UserInterface|GetUserWidgetObject (Variables|Default|GetHealthWidget))))
      (Variables|/Game/UserInteface/WBP_ZombieHealth.WBP_ZombieHealth_C|SetZombieRef _aswbp_zombie_health self))
    (:then_1
      (Rendering|SetVisibility (Variables|Default|GetHealthWidget) false false))))

(event EventTick
  (params (DeltaSeconds :type Float%20%28single-precision%29))
  ;[0.15 0.15 0.15 0.5] // Health Bar Location
  (Transformation|SetWorldRotation (Variables|Default|GetHealthWidget) (Math|Rotator|FindLookatRotation (Transformation|GetWorldLocation (Variables|Default|GetHealthWidget)) (Camera|GetCameraLocation (Game|GetPlayerCameraManager 0))) false false))

(fn ConstructionScript)

(fn ApplyHealthDamage
  (params (Delta :type Float%20%28double-precision%29))
  (bind _output_get (Variables|Default|SetHealth (Math|Float|Clamp(Float) (+ (Variables|Default|GetHealth) Delta) 0.0 (Variables|Default|GetMaxHealth))))
  (if (<= _output_get 0.0)
    (if (not (Variables|Default|GetIsDead))
      (CallFunction|Die))))