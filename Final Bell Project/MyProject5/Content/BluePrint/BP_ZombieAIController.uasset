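; AI controller for zombies that chases the player on sight and attacks at close range.
; AI Perception updates player visibility and the target reference, while a looping timer set on BeginPlay drives the chase check instead of Tick.
; Within a fixed distance the zombie stops, yaws toward the player and starts its attack; it halts when sight is lost or the player dies.
; An unconnected AttackRange-based chase variant remains, noted as broken.
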(event OnTargetPerceptionUpdated(AIPerception)
  (params (Actor :type Actor%20Object%20Reference) (Stimulus :type AI%20Stimulus%20Structure))
  (bind _asbp_third_person_character (Utilities|Casting|CastToBP_ThirdPersonCharacter Actor))
  (bind _output_get (Variables|Default|SetCanSeePlayer (.bSuccessfullySensed (Utilities|Struct|BreakAIStimulus Stimulus))))
  (if _output_get
    (Variables|Default|SetPlayerRef _asbp_third_person_character)
    (else
      (Variables|Default|SetPlayerRef 0))))

(event Custom|ChasePlayer
  (bind _returnvalue (Pawn|GetControlledPawn))
  (bind _playerref (Variables|Default|GetPlayerRef))
  (bind _asbp_third_person_character (Utilities|Casting|CastToBP_ThirdPersonCharacter (Game|GetPlayerCharacter 0)))
  (if (Variables|/Game/ThirdPerson/Blueprints/BP_ThirdPersonCharacter.BP_ThirdPersonCharacter_C|GetisDead _asbp_third_person_character)
    (Utilities|Time|ClearandInvalidateTimerbyHandle (Variables|Default|GetChaseTimerHandle))
    (AI|Navigation|StopMovement)
    (elif (Variables|Default|GetCanSeePlayer)
      (if (<= (Math|Vector|Distance(Vector) (Transformation|GetActorLocation _returnvalue) (Transformation|GetActorLocation _playerref)) 1.5e+02)
        (AI|Navigation|StopMovement)
        (Transformation|SetActorRotation (Pawn|GetControlledPawn) (Math|Rotator|MakeRotator 0.0 0.0 (.Yaw (Math|Rotator|BreakRotator (Math|Rotator|FindLookatRotation (Transformation|GetActorLocation (Pawn|GetControlledPawn)) (Transformation|GetActorLocation (Variables|Default|GetPlayerRef)))))))
        (bind _asbp_zombie (Utilities|Casting|CastToBP_Zombie _returnvalue))
        (if (and (not (Variables|/Game/BluePrint/BP_Zombie.BP_Zombie_C|GetIsAttacking _asbp_zombie)) (not (Variables|/Game/BluePrint/BP_Zombie.BP_Zombie_C|GetIsDead _asbp_zombie)))
          (Default|StartAttack _asbp_zombie))
        (else
          (AI|AIMoveTo 0 "0, 0, 0" _playerref 1e+02 true)))
      (else
        (AI|Navigation|StopMovement)))))

(event EventBeginPlay
  (Utilities|FlowControl|Sequence
    (:then_0
      (bind _returnvalue (Utilities|Time|SetTimerbyEvent (EventDispatchers|CreateEvent :!event Custom|ChasePlayer) 0.2 true))
      (Variables|Default|SetChaseTimerHandle _returnvalue))
    (:then_1
      (bind _asbp_third_person_character (Utilities|Casting|CastToBP_ThirdPersonCharacter (Game|GetPlayerCharacter 0)))
      (Variables|Default|SetPlayerRef _asbp_third_person_character))))

(event EventTick
  (params (DeltaSeconds :type Float%20%28single-precision%29)))

(fn ConstructionScript)