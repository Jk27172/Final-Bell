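; BP_FireAxeCase is an interactable fire axe case that the player can break once by pressing E nearby.
; It enables input from player controller 0 on BeginPlay, and InteractBox overlaps toggle a PlayerInside flag without filtering the overlapping actor.
; Pressing E inside the box sets Broken, hides StaticMeshComponent0, disables its collision and plays a glass-break sound at the actor's location.
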(event OnComponentBeginOverlap(InteractBox)
  (params (OverlappedComponent :type Primitive%20Component%20Object%20Reference) (OtherActor :type Actor%20Object%20Reference) (OtherComp :type Primitive%20Component%20Object%20Reference) (OtherBodyIndex :type Integer) (bFromSweep :type Boolean) (SweepResult :type Hit%20Result%20Structure%20%28by%20ref%29))
  (Variables|Default|SetbPlayerInside true))

(event OnComponentEndOverlap(InteractBox)
  (params (OverlappedComponent :type Primitive%20Component%20Object%20Reference) (OtherActor :type Actor%20Object%20Reference) (OtherComp :type Primitive%20Component%20Object%20Reference) (OtherBodyIndex :type Integer))
  (Variables|Default|SetbPlayerInside false))

(event EventBeginPlay
  (Input|EnableInput (Game|GetPlayerController 0)))

(event Collision|EventActorBeginOverlap
  (params (OtherActor :type Actor%20Object%20Reference)))

(event EventTick
  (params (DeltaSeconds :type Float%20%28single-precision%29)))

(event Input|KeyboardEvents|E
  (params (Key :type Key%20Structure))
  (:Pressed
    (if (Variables|Default|GetbPlayerInside)
      (if (not (Variables|Default|GetbBroken))
        (Variables|Default|SetbBroken true)
        (Rendering|SetVisibility (Variables|Default|GetStaticMeshComponent0) false false)
        (Collision|SetCollisionEnabled (Variables|Default|GetStaticMeshComponent0) "NoCollision")
        (Audio|PlaySoundatLocation "/Game/Import/Sound/479449__rogeriobiadola__glass-break.479449__rogeriobiadola__glass-break" (Transformation|GetActorLocation) "0, 0, 0" 1.0 1.0 0.0 0 0 0 0)))))

(fn ConstructionScript)